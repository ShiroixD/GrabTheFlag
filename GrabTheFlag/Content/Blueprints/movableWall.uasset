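; Moving wall actor that travels along a spline taken from a referenced platform actor.
; On BeginPlay it records its start location and, when active and on the server authority, starts a timeline whose rate comes from a duration and whose start time comes from an offset.
; Each update maps the timeline alpha to a distance on that spline and adds the local-space point to the start location.
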(event Custom|MovePlatform
  (Components|Timeline|SetPlayRate (Variables|Default|GetPlatformMover) (/ 1.0 (Variables|Default|GetDuration)))
  (Components|Timeline|SetNewTime (Variables|Default|GetPlatformMover) (Variables|Default|GetPlatformStartOffset))
  (bind _alpha (Timeline|PlatformMover Play)
    (:Update
      (Variables|Default|SetAlpha _alpha)
      (Transformation|SetActorLocation (+ (Spline|GetLocationatDistanceAlongSpline (Variables|/Game/Blueprints/Track.Track_C|GetUsefulSpline (Variables|Default|GetPlatformRef)) (Math|Float|Lerp 0.0 (Spline|GetSplineLength (Variables|/Game/Blueprints/Track.Track_C|GetUsefulSpline (Variables|Default|GetPlatformRef))) (Variables|Default|GetAlpha)) "Local") (Variables|Default|GetStartingLocation)) false false))))

(event EventBeginPlay
  (Variables|Default|SetStartingLocation (Transformation|GetActorLocation))
  (if (Variables|Default|GetActivePlatform)
    (Networking|SwitchHasAuthority
      (:Authority
        (CallFunction|MovePlatform)))))

(fn ConstructionScript)