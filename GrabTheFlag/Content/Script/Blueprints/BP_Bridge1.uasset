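; BP_Bridge1 is a bridge actor that moves along a timeline-driven path from its placed position.
; On BeginPlay, only the authority stores the start location and plays Timeline_0.
; Each timeline update adds the Move track to that start location and calls a move event, which sets the actor location without sweeping.
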(event Custom|Move_Event
  (Transformation|SetActorLocation (Variables|Default|GetNewLoc) false false))

(event EventBeginPlay
  (Networking|SwitchHasAuthority
    (:Authority
      (Variables|Default|SetStartLoc (Transformation|GetActorLocation))
      (bind _move (Timeline|Timeline_0 PlayFromStart)
        (:Update
          (Variables|Default|SetNewLoc (+ _move (Variables|Default|GetStartLoc)))
          (CallFunction|MoveEvent))))))

(event Collision|EventActorBeginOverlap
  (params (OtherActor :type Actor%20Object%20Reference)))

(fn ConstructionScript)