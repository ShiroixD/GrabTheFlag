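; BP_Bridge12 is an actor, named as a bridge, that moves along a timeline-driven offset from its starting location.
; On BeginPlay, only the authority records the start location and plays the timeline from the start.
; Each update adds the timeline's Move value to that location and calls MoveEvent.
; A custom event sets the actor location to the computed position without sweeping.
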(event Custom|CustomEvent
  (Transformation|SetActorLocation (Variables|Default|GetNewLoc) false false))

(event EventBeginPlay
  (Networking|SwitchHasAuthority
    (:Authority
      (Variables|Default|SetStartLoc (Transformation|GetActorLocation))
      (bind _move (Timeline|Timeline_1 PlayFromStart)
        (:Update
          (Variables|Default|SetNewLoc (+ _move (Variables|Default|GetStartLoc)))
          (CallFunction|MoveEvent))))))

(event Collision|EventActorBeginOverlap
  (params (OtherActor :type Actor%20Object%20Reference))
  (|CallParentFunction OtherActor) ; This node is disabled and will not be called.\nDrag off pins to build functionality.
)

(event EventTick
  (params (DeltaSeconds :type Float%20%28single-precision%29)))

(fn ConstructionScript
  (|CallParentFunction))