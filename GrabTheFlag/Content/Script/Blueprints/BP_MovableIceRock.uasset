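; BP_MovableIceRock is an ice rock actor that moves along a timeline-driven path relative to its starting location.
; On BeginPlay, only the authority stores the actor's location and plays the timeline from the start.
; Each update adds the Movement track to that origin and calls a move event, which sets the location without sweep or teleport.
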(event Custom|Move_Event
  (Transformation|SetActorLocation (Variables|Default|GetNewLoc) false false))

(event EventBeginPlay
  (Networking|SwitchHasAuthority
    (:Authority
      (Variables|Default|SetNewLocation (Transformation|GetActorLocation))
      (bind _movement (Timeline|Timeline_0 PlayFromStart)
        (:Update
          (Variables|Default|SetNewLoc (+ _movement (Variables|Default|GetNewLocation)))
          (CallFunction|MoveEvent))))))

(event Collision|EventActorBeginOverlap
  (params (OtherActor :type Actor%20Object%20Reference)))

(event EventTick
  (params (DeltaSeconds :type Float%20%28single-precision%29)))

(fn ConstructionScript)