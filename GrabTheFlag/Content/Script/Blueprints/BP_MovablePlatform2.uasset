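; BP_MovablePlatform2 is a moving platform that follows a timeline-driven offset from its starting location.
; On BeginPlay, only the authority stores the initial location and plays the timeline from the start.
; Each timeline update adds the Movement value to that location and calls a custom event that sets the actor's position without sweeping.
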(event Custom|Movw_Event
  (Transformation|SetActorLocation (Variables|Default|GetNewLoc_0) false false))

(event EventBeginPlay
  (Networking|SwitchHasAuthority
    (:Authority
      (Variables|Default|SetInitLocation2_0 (Transformation|GetActorLocation))
      (bind _movement (Timeline|Timeline_0 PlayFromStart)
        (:Update
          (Variables|Default|SetNewLoc_0 (+ _movement (Variables|Default|GetInitLocation2_0)))
          (CallFunction|MovwEvent))))))

(event Collision|EventActorBeginOverlap
  (params (OtherActor :type Actor%20Object%20Reference))
  (|CallParentFunction OtherActor) ; This node is disabled and will not be called.\nDrag off pins to build functionality.
)

(event EventTick
  (params (DeltaSeconds :type Float%20%28single-precision%29))
  (|CallParentFunction DeltaSeconds) ; This node is disabled and will not be called.\nDrag off pins to build functionality.
)

(fn ConstructionScript
  (|CallParentFunction))