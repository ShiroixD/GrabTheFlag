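; Bonus is a pickup actor that picks a random type from six options on BeginPlay.
; When a ThirdPersonCharacter overlaps its box, it sets that character's BonusType and HasFlag.
; It then passes its transform to the BonusGenerator actors through AddElemnt, destroys itself, and plays a pickup sound and explosion effect.
; The switch on bonus type has only empty branches.
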(event OnComponentBeginOverlap(Box)
  (params (OverlappedComponent :type Primitive%20Component%20Object%20Reference) (OtherActor :type Actor%20Object%20Reference) (OtherComp :type Primitive%20Component%20Object%20Reference) (OtherBodyIndex :type Integer) (bFromSweep :type Boolean) (SweepResult :type Hit%20Result%20Structure%20%28by%20ref%29))
  (bind _returnvalue (Transformation|GetActorLocation))
  (bind _asthird_person_character (Utilities|Casting|CastToThirdPersonCharacter OtherActor))
  (Variables|/Game/ThirdPersonBP/Blueprints/ThirdPersonCharacter.ThirdPersonCharacter_C|SetBonusType _asthird_person_character (Variables|Default|GetBonusType))
  (Variables|/Game/ThirdPersonBP/Blueprints/ThirdPersonCharacter.ThirdPersonCharacter_C|SetHasFlag _asthird_person_character true)
  (bind _outactors (Actor|GetAllActorsOfClass "/Game/Script/Blueprints/BonusGenerator.BonusGenerator_C"))
  (Default|AddElemnt _outactors (Transformation|GetActorTransform self))
  (switch int (Variables|Default|GetBonusType)
    (:Default
      _)
    (:0
      _)
    (:1
      _)
    (:2
      _)
    (:3
      _)
    (:4
      _)
    (:5
      _))
  (Actor|DestroyActor)
  (Audio|PlaySoundatLocation "/Game/Picked_Coin_Echo_2.Picked_Coin_Echo_2" _returnvalue "0, 0, 0" 1.0 1.0 0.0 0 0 0)
  (Effects|SpawnEmitteratLocation "/Game/StarterContent/Particles/P_Explosion.P_Explosion" _returnvalue))

(event EventBeginPlay
  (Variables|Default|SetBonusType (Math|Random|RandomIntegerinRange 0 5)))

(event EventTick
  (params (DeltaSeconds :type Float%20%28single-precision%29)))

(fn ConstructionScript)