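; BonusGenerator is an actor that spawns Bonus objects at random free spawn points.
; BeginPlay caches the transforms of the SpawnObcject actors in SpawnPosition.
; A Delay on Tick calls GenerateBonus about every five seconds, spawning at a random stored transform and removing it so it is not reused.
; AddElemnt can add transforms back to the pool, while the counter-driven Loop function is not called within this graph.
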(event EventBeginPlay
  (for _array_element (Variables|Default|GetSpawnObcject)
    (Utilities|Array|Add (Variables|Default|GetSpawnPosition) (Transformation|GetActorTransform _array_element))))

(event Collision|EventActorBeginOverlap
  (params (OtherActor :type Actor%20Object%20Reference)))

(event EventTick
  (params (DeltaSeconds :type Float%20%28single-precision%29))
  (Utilities|FlowControl|Delay 5.0)
  (CallFunction|GenerateBonus))

(fn ConstructionScript)

(fn GenerateBonus
  (if (!= (Utilities|Array|Length (Variables|Default|GetSpawnPosition)) 0)
    (Variables|Default|SetRandomHelp (Math|Random|RandomIntegerinRange 0 (- (Utilities|Array|Length (Variables|Default|GetSpawnPosition)) 1)))
    (Game|SpawnActorfromClass "/Game/Script/Blueprints/Bonus.Bonus_C" (Utilities|Array|Get(acopy) (Variables|Default|GetSpawnPosition) (Variables|Default|GetRandomHelp)) "Undefined" 0 0)
    (Utilities|Array|RemoveIndex (Variables|Default|GetSpawnPosition) (Variables|Default|GetRandomHelp))))

(fn Loop
  ;[1 1 1] Loop generete obcject
  (while (Variables|Default|Getbool)
    (CallFunction|GenerateBonus)
    (if (== (Variables|Default|Getint) 1)
      (Variables|Default|Setbool false)
      (else
        (Variables|Default|Setint (+ (Variables|Default|Getint) 1)))))
  (Development|PrintString "Hello2"))

(fn AddElemnt
  (params (trans :type Transform))
  (Utilities|Array|Add (Variables|Default|GetSpawnPosition) trans))