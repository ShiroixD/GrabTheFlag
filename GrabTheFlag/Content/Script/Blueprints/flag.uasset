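; Flag pickup actor that a ThirdPersonCharacter collects by touching it.
; On collider overlap with that exact class, it snaps onto the character mesh's "fs" socket, disables its own collision and shrinks.
; It then ends its particle trails and sets HasFlag on the character.
; The file contains no drop or reset logic.
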(event OnComponentBeginOverlap(colider)
  (params (OverlappedComponent :type Primitive%20Component%20Object%20Reference) (OtherActor :type Actor%20Object%20Reference) (OtherComp :type Primitive%20Component%20Object%20Reference) (OtherBodyIndex :type Integer) (bFromSweep :type Boolean) (SweepResult :type Hit%20Result%20Structure%20%28by%20ref%29))
  (if (== "/Game/ThirdPersonBP/Blueprints/ThirdPersonCharacter.ThirdPersonCharacter_C" (Utilities|GetClass OtherActor))
    (bind _asthird_person_character (Utilities|Casting|CastToThirdPersonCharacter OtherActor))
    (Variables|Default|Setthird _asthird_person_character)
    (Transformation|AttachComponentToComponent (Variables|/Script/Engine.Character|GetMesh (Variables|Default|Getthird)) "fs" "SnapToTarget" "SnapToTarget" "SnapToTarget" true)
    (Collision|SetActorEnableCollision false)
    (Transformation|SetActorRelativeScale3D "0.400000,0.400000,0.400000")
    (Effects|Particles|Trails|EndTrails (Variables|Default|GetParticleSystem))
    (Variables|/Game/ThirdPersonBP/Blueprints/ThirdPersonCharacter.ThirdPersonCharacter_C|SetHasFlag (Variables|Default|Getthird) true)))

(event EventBeginPlay)

(event Collision|EventActorBeginOverlap
  (params (OtherActor :type Actor%20Object%20Reference)))

(event EventTick
  (params (DeltaSeconds :type Float%20%28single-precision%29)))

(fn ConstructionScript)